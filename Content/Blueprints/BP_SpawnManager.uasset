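; BP_SpawnManager runs endless enemy waves, voicing a villain through on-screen debug taunts.
; Shortly after BeginPlay, SpawnEnemies visits every BP_Spawnpoint and spawns a BP_Enemy at each on a weighted random roll.
; Dying enemies are meant to call WaveCheck, which counts remaining BP_Enemy actors and starts a new wave after a delay when at most one is left.
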(event `self.ReceiveBeginPlay`
  (`KismetSystemLibrary.PrintString` "You'll never get the Cubes!" true true (struct :`R` 1.0 :`B` 0.007519 :`A` 1.0))
  (`KismetSystemLibrary.Delay` 1.0)
  (`self.Spawn Enemies`))

(event `Spawn Enemies`
  (bind _outactors (`GameplayStatics.GetAllActorsOfClass` "/Game/Blueprints/BP_Spawnpoint.BP_Spawnpoint_C"))
  (for _array_element _outactors
    (`KismetSystemLibrary.PrintString` (`KismetSystemLibrary.GetDisplayName` _array_element) true true (struct :`R` 1.0 :`B` 0.007629 :`A` 1.0) 8.0)
    (if (`KismetMathLibrary.RandomBoolWithWeight` 0.8)
      (`|SpawnActorFromClass` "/Game/Blueprints/BP_Enemy.BP_Enemy_C" (`SceneComponent.K2_GetComponentToWorld` (`/Game/Blueprints/BP_Spawnpoint.DefaultSceneRoot` _array_element)) "Undefined" "MultiplyWithRoot" null null)))
  (`KismetSystemLibrary.PrintString` "Get them my minions!" true true (struct :`R` 1.0 :`G` 0.007892 :`A` 1.0)))

(event `Wave Check`
  (`KismetSystemLibrary.PrintString` "My minions never yield!" true true (struct :`R` 1.0 :`B` 0.015508 :`A` 1.0))
  (bind _outactors (`GameplayStatics.GetAllActorsOfClass` "/Game/Blueprints/BP_Enemy.BP_Enemy_C"))
  (bind _returnvalue (`KismetArrayLibrary.Array_Length` _outactors))
  (`KismetSystemLibrary.PrintString` (`KismetStringLibrary.Concat_StrStr` "ARRGH I only have" (`KismetStringLibrary.Conv_IntToString` _returnvalue) "Minions left") true true (struct :`R` 1.0 :`G` 0.050841 :`A` 1.0))
  (if (> _returnvalue 1)
    (`KismetSystemLibrary.PrintString` "Fight with all you have my minions!")
    (else
      (`KismetSystemLibrary.Delay` 3.0)
      (`self.Spawn Enemies`))))

(fn `UserConstructionScript`)